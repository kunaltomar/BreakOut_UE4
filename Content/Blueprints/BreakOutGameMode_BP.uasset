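; BreakOutGameMode_BP is the game mode for a Breakout game, driving the HUD's menu and game-start states.
; On BeginPlay it calls ShowMenu, which creates and caches the BreakOut_HUD widget if none exists, then calls ResetLevel on it.
; HideHintText calls StartTheGame on the cached HUD when it is valid.
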(event `self.ReceiveBeginPlay`
  (`self.ShowMenu`))

(event `self.ShowMenu`
  (`/Engine/EditorBlueprintResources/StandardMacros.IsValid` (`self.HUD_ref`)
    (:`Is Valid`
      (`/Game/UI/BreakOut_HUD.ResetLevel` (`self.HUD_ref`)))
    (:`Is Not Valid`
      (bind _returnvalue (`|CreateWidget` "/Game/UI/BreakOut_HUD.BreakOut_HUD_C"))
      (bind _output_get (set `self.HUD_ref` _returnvalue))
      (`UserWidget.AddToViewport` _output_get 0)
      (`/Game/UI/BreakOut_HUD.ResetLevel` _output_get))))

(event `HideHintText`
  (`/Engine/EditorBlueprintResources/StandardMacros.IsValid` (`self.HUD_ref`)
    (:`Is Valid`
      (`/Game/UI/BreakOut_HUD.StartTheGame` (`self.HUD_ref`)))))

(fn `UserConstructionScript`)